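; BPCharacter is a flipbook-sprite fighter character, handled as player 1, that turns to face its opponent, BPCharacter2.
; BeginPlay sets the sprite to replicate and caches the opponent and MyPlayerController1.
; Each Tick picks the secret agent flipbook from ActionState and velocity, then sets control yaw by comparing X positions with a freshly looked-up opponent.
; Landing is forwarded to MyPlayerController1 through OnLandedPlayer1.
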(event `UpdateAnimation`
  (params (ActionState :type "/Game/ShooterFighter/Blueprints/Char_States Enum" :default "NewEnumerator0"))
  ;[1 1 1] Handle Animation
  (bind _output_get (set `self.ActionState` ActionState))
  (switch `/Game/ShooterFighter/Blueprints/Char_States` _output_get
    (:`NewEnumerator0`
      (`PaperFlipbookComponent.SetFlipbook` (`self.Sprite`) (select `bool` (> (`KismetMathLibrary.VSize` (`self.GetVelocity`)) 0.0) :`false` "/Game/ShooterFighter/Sprites/Flipbooks/SecretAgent/FB_Secret_Agent_Idle.FB_Secret_Agent_Idle" :`true` "/Game/ShooterFighter/Sprites/Flipbooks/SecretAgent/FB_Secret_Agent_running.FB_Secret_Agent_running" :!type "PaperFlipbook Object Reference")))
    (:`NewEnumerator1`
      (`PaperFlipbookComponent.SetFlipbook` (`self.Sprite`) "/Game/ShooterFighter/Sprites/Flipbooks/SecretAgent/FB_Secret_Agent_running.FB_Secret_Agent_running"))
    (:`NewEnumerator2`
      (`PaperFlipbookComponent.SetFlipbook` (`self.Sprite`) "/Game/ShooterFighter/Sprites/Flipbooks/SecretAgent/FB_Secret_Agent_jumping.FB_Secret_Agent_jumping"))))

(event `self.ReceiveBeginPlay`
  (`|ExecutionSequence`
    (:`then_0`
      (`ActorComponent.SetIsReplicated` (`self.Sprite`) true))
    (:`then_1`
      (bind _outactors (`GameplayStatics.GetAllActorsOfClass` "/Game/ShooterFighter/Blueprints/BPCharacter2.BPCharacter2_C"))
      (set `self.Char2` (`|GetArrayItem` _outactors)))
    (:`then_2`
      (bind _outactors_2 (`GameplayStatics.GetAllActorsOfClass` "/Game/ShooterFighter/Blueprints/MyPlayerController1.MyPlayerController1_C"))
      (set `self.PlayerController1` (`|GetArrayItem` _outactors_2)))))

(event `self.ReceiveTick`
  (params (DeltaSeconds :type "Float (single-precision)"))
  ;[1 1 1] Tick - Updates animation
  (`self.UpdateAnimation` (`self.ActionState`))
  (bind _outactors (`GameplayStatics.GetAllActorsOfClass` "/Game/ShooterFighter/Blueprints/BPCharacter2.BPCharacter2_C"))
  (`/Engine/EditorBlueprintResources/StandardMacros.CompareFloat` (- (.x (`self.K2_GetActorLocation`)) (.x (`self.K2_GetActorLocation` (`|GetArrayItem` _outactors))))
    (:`>`
      (`Controller.SetControlRotation` (`self.GetController`) (`KismetMathLibrary.MakeRotator` 0.0 0.0 180.0)))
    (:`<`
      (`Controller.SetControlRotation` (`self.GetController`) (`KismetMathLibrary.MakeRotator` 0.0)))))

(event `self.OnLanded`
  (params (Hit :type "HitResult Structure (by ref)"))
  ;[1 1 1] Handle Jump
  (bind _asmy_player_controller_1 (cast `/Game/ShooterFighter/Blueprints/MyPlayerController1` (`self.GetController`)))
  (`/Game/ShooterFighter/Blueprints/MyPlayerController1.OnLandedPlayer1` _asmy_player_controller_1))

(fn `UserConstructionScript`)