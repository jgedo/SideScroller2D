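; Player controller for a local two-player shooter fighter that runs both players from one keyboard, spawning Player 2's controller and character on BeginPlay.
; It handles movement, jumping, shooting with reloads, pausing, and tracks health, ammo and round wins in a per-character struct.
; Key presses feed timed three-key input chains, matched against each player's combo list.
; A match facing the opponent, judged by relative X position, fires a double-shot special.
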(event `Key|BackSpace`
  (params (Key :type "Key Structure"))
  (bind _returnvalue (`GameplayStatics.GetPlayerController` 0))
  ;[1 1 1] Pause Game
  (:`Pressed`
    (if (`self.InputEnabled`)
      (`GameplayStatics.SetGamePaused` true)
      (bind _foundwidgets (`WidgetBlueprintLibrary.GetAllWidgetsOfClass` "/Game/ShooterFighter/HUD/InGameMenuUI.InGameMenuUI_C"))
      (bind _output (`|GetArrayItem` _foundwidgets))
      (`Widget.SetVisibility` _output "Visible")
      (`WidgetBlueprintLibrary.SetInputMode_UIOnlyEx` _returnvalue _output "LockAlways")
      (set `PlayerController.bShowMouseCursor` true _returnvalue))))

(event `UpdateInputEnabled`
  (params (InputEnabled :type Boolean))
  ;[1 1 1] Update Input Enabled
  (set `self.InputEnabled` InputEnabled))

(event `self.ReceiveBeginPlay`
  (bind _returnvalue (`KismetMathLibrary.MakeTransform` (250.0 495.0 152.0)))
  (`|ExecutionSequence`
    (:`then_0`
      ;[1 1 1] Set Up Player 2
      (bind _returnvalue_2 (`|SpawnActorFromClass` "/Game/ShooterFighter/Blueprints/MyPlayerController2.MyPlayerController2_C" _returnvalue "Undefined" "OverrideRootScale" null null))
      (set `self.Char2Controller` _returnvalue_2)
      (bind _returnvalue_3 (`|SpawnActorFromClass` "/Game/ShooterFighter/Blueprints/BPCharacter2.BPCharacter2_C" _returnvalue "Undefined" "OverrideRootScale" null null))
      (set `self.Char2` _returnvalue_3))
    (:`then_1`
      (bind _outactors (`GameplayStatics.GetAllActorsOfClass` "/Game/ShooterFighter/Blueprints/BPCharacter.BPCharacter_C"))
      (set `self.Char1` (`|GetArrayItem` _outactors)))))

(event `self.ReceiveTick`
  (params (DeltaSeconds :type "Float (single-precision)"))
  (bind _char2info (`self.Char2Info`))
  (bind _char1info (`self.Char1Info`))
  (`|ExecutionSequence`
    (:`then_0`
      (setmembers `/Game/ShooterFighter/Blueprints/Structs/CharStruct` :`StructRef` _char1info :`SpecialTimer` (- (`.SpecialTimer_12_4734324540203F26D7FC7C812F8E0032` (break `/Game/ShooterFighter/Blueprints/Structs/CharStruct` _char1info)) DeltaSeconds)))
    (:`then_1`
      (setmembers `/Game/ShooterFighter/Blueprints/Structs/CharStruct` :`StructRef` _char2info :`SpecialTimer` (- (`.SpecialTimer_12_4734324540203F26D7FC7C812F8E0032` (break `/Game/ShooterFighter/Blueprints/Structs/CharStruct` _char2info)) DeltaSeconds)))))

(event `SpecialMove1_P1`
  ;[1 1 1] Special Shot P1
  (`self.SpecialShotP1`))

(event `UpdateAmmoP1`
  (bind _char1info (`self.Char1Info`))
  (bind (_movingr _shooting _reloading _firerate _reloadtime _specialtimer _sm _inputchain _maxhealth _health _maxammo _currentammo) (break `/Game/ShooterFighter/Blueprints/Structs/CharStruct` _char1info))
  ;[1 1 1] Update Ammo Player 1
  (bind _structout (setmembers `/Game/ShooterFighter/Blueprints/Structs/CharStruct` :`StructRef` _char1info :`CurrentAmmo` (- _currentammo 1)))
  (`/Engine/EditorBlueprintResources/StandardMacros.CompareInt` (`.CurrentAmmo_28_752318D44ED93FAD5F9156BBE02568EF` (break `/Game/ShooterFighter/Blueprints/Structs/CharStruct` _structout))
    (:`==`
      (setmembers `/Game/ShooterFighter/Blueprints/Structs/CharStruct` :`StructRef` _char1info :`Reloading` true)
      (`KismetSystemLibrary.Delay` _reloadtime)
      (setmembers `/Game/ShooterFighter/Blueprints/Structs/CharStruct` :`StructRef` _char1info :`Reloading` false :`CurrentAmmo` _maxammo))))

(event `SpecialShotP1`
  (bind _char1info (`self.Char1Info`))
  (bind _returnvalue (`SceneComponent.K2_GetComponentToWorld` (`/Game/ShooterFighter/Blueprints/BPCharacter.ArrowShot` (`self.Char1`))))
  ;[1 1 1] Special Shot P1
  (if (`self.InputEnabled`)
    (if (not (`.Reloading_5_2516DC3643F2DA088FF503800CA586F7` (break `/Game/ShooterFighter/Blueprints/Structs/CharStruct` (`self.Char1Info`))))
      (`|ExecutionSequence`
        (:`then_0`
          (`GameplayStatics.PlaySoundAtLocation` "/Game/ShooterFighter/Sound/Effects/S_Gunshot.S_Gunshot" (0.0 0.0 0.0) (struct) 0.6)
          (`|SpawnActorFromClass` "/Game/ShooterFighter/Blueprints/BP_Bullet.BP_Bullet_C" _returnvalue "Undefined" "OverrideRootScale" null null)
          (`self.UpdateAmmoP1`)
          (`KismetSystemLibrary.Delay` 0.15)
          (`GameplayStatics.PlaySoundAtLocation` "/Game/ShooterFighter/Sound/Effects/S_Gunshot.S_Gunshot" (0.0 0.0 0.0) (struct) 0.6)
          (`|SpawnActorFromClass` "/Game/ShooterFighter/Blueprints/BP_Bullet.BP_Bullet_C" _returnvalue "Undefined" "OverrideRootScale" null null)
          (setmembers `/Game/ShooterFighter/Blueprints/Structs/CharStruct` :`StructRef` _char1info :`Shooting` true)
          (`KismetSystemLibrary.Delay` (+ (`.FireRate_8_44F8AAA74B17C0093544B193761FC9C2` (break `/Game/ShooterFighter/Blueprints/Structs/CharStruct` _char1info)) 0.15))
          (setmembers `/Game/ShooterFighter/Blueprints/Structs/CharStruct` :`StructRef` (`self.Char1Info`) :`Shooting` false))))))

(event `Key|G`
  (params (Key :type "Key Structure"))
  (bind _char1info (`self.Char1Info`))
  (bind (_movingr _shooting _reloading) (break `/Game/ShooterFighter/Blueprints/Structs/CharStruct` (`self.Char1Info`)))
  ;[1 1 1] Shooting
  (:`Pressed`
    (`self.SetInputChainP1` Key)
    (if (and (`self.InputEnabled`) (not _shooting) (not _reloading))
      (`|ExecutionSequence`
        (:`then_0`
          (`GameplayStatics.PlaySoundAtLocation` "/Game/ShooterFighter/Sound/Effects/S_Gunshot.S_Gunshot" (0.0 0.0 0.0) (struct) 0.6))
        (:`then_1`
          (`|SpawnActorFromClass` "/Game/ShooterFighter/Blueprints/BP_Bullet.BP_Bullet_C" (`SceneComponent.K2_GetComponentToWorld` (`/Game/ShooterFighter/Blueprints/BPCharacter.ArrowShot` (`self.Char1`))) "Undefined" "OverrideRootScale" null null))
        (:`then_2`
          (`self.UpdateAmmoP1`))
        (:`then_3`
          (setmembers `/Game/ShooterFighter/Blueprints/Structs/CharStruct` :`StructRef` _char1info :`Shooting` true)
          (`KismetSystemLibrary.Delay` (`.FireRate_8_44F8AAA74B17C0093544B193761FC9C2` (break `/Game/ShooterFighter/Blueprints/Structs/CharStruct` _char1info)))
          (setmembers `/Game/ShooterFighter/Blueprints/Structs/CharStruct` :`StructRef` (`self.Char1Info`) :`Shooting` false))))))

(event `Key|A`
  (params (Key :type "Key Structure"))
  ;[1 1 1] P1 Input Chains
  (:`Pressed`
    (`self.SetInputChainP1` Key)))

(event `InputAction|Jump`
  (params (Key :type "Key Structure"))
  (bind _char1 (`self.Char1`))
  (bind _inputenabled (`self.InputEnabled`))
  ;[1 1 1] Handle Jump
  (:`Pressed`
    (if _inputenabled
      (`Character.Jump` _char1)
      (bind _output_get (set `self.ActionState` "NewEnumerator2"))
      (`/Game/ShooterFighter/Blueprints/BPCharacter.UpdateAnimation` _char1 _output_get)))
  (:`Released`
    (if _inputenabled
      (`Character.StopJumping` _char1))))

(event `InputAxis|MoveRight`
  (params (AxisValue :type "Float (single-precision)"))
  (bind _returnvalue (`self.K2_GetPawn`))
  ;[1 1 1] Handle movement
  (if (`self.InputEnabled`)
    (cast `/Game/ShooterFighter/Blueprints/BPCharacter` _returnvalue)
    (`Pawn.AddMovementInput` _returnvalue (1.0 0.0 0.0) AxisValue false)))

(event `Key|S`
  (params (Key :type "Key Structure"))
  ;[1 1 1] P1 Input Chains
  (:`Pressed`
    (`self.SetInputChainP1` Key)))

(event `Key|D`
  (params (Key :type "Key Structure"))
  ;[1 1 1] P1 Input Chains
  (:`Pressed`
    (`self.SetInputChainP1` Key)))

(event `DamageP1`
  (params (Damage :type "Float (double-precision)"))
  (bind _char1info (`self.Char1Info`))
  ;[1 1 1] Damage Player 1
  (setmembers `/Game/ShooterFighter/Blueprints/Structs/CharStruct` :`StructRef` _char1info :`Health` (- (`.Health_23_413A2251404E3EBFA307E59EFC07D439` (break `/Game/ShooterFighter/Blueprints/Structs/CharStruct` _char1info)) Damage)))

(event `Respawn P1`
  (bind _char1info (`self.Char1Info`))
  (bind (_movingr _shooting _reloading _firerate _reloadtime _specialtimer _sm _inputchain _maxhealth _health _maxammo) (break `/Game/ShooterFighter/Blueprints/Structs/CharStruct` _char1info))
  ;[1 1 1] Respawn Player 1
  (setmembers `/Game/ShooterFighter/Blueprints/Structs/CharStruct` :`StructRef` _char1info :`Health` _maxhealth :`CurrentAmmo` _maxammo))

(event `OnLandedPlayer1`
  ;[1 1 1] Handle Jump
  (bind _output_get (set `self.ActionState` "NewEnumerator0"))
  (`/Game/ShooterFighter/Blueprints/BPCharacter.UpdateAnimation` (`self.Char1`) _output_get))

(event `UpdateWinsP1`
  (bind _char1info (`self.Char1Info`))
  ;[1 1 1] Update Wins P1
  (setmembers `/Game/ShooterFighter/Blueprints/Structs/CharStruct` :`StructRef` _char1info :`CurrentWins` (+ (`.CurrentWins_30_FD63D54E4C90841E1CCF2E9FCAE436A6` (break `/Game/ShooterFighter/Blueprints/Structs/CharStruct` _char1info)) 1))
  (set `self.Round` (+ (`self.Round`) 1)))

(event `Key|W`
  (params (Key :type "Key Structure"))
  ;[1 1 1] P1 Input Chains
  (:`Pressed`
    (`self.SetInputChainP1` Key)))

(event `SpecialMove1_P2`
  ;[1 1 1] Special Shot P2
  (`self.SpecialShotP2`))

(event `UpdateAmmoP2`
  (bind _char2info (`self.Char2Info`))
  (bind (_movingr _shooting _reloading _firerate _reloadtime _specialtimer _sm _inputchain _maxhealth _health _maxammo _currentammo) (break `/Game/ShooterFighter/Blueprints/Structs/CharStruct` _char2info))
  ;[1 1 1] Update Ammo Player 2
  (bind _structout (setmembers `/Game/ShooterFighter/Blueprints/Structs/CharStruct` :`StructRef` _char2info :`CurrentAmmo` (- _currentammo 1)))
  (`/Engine/EditorBlueprintResources/StandardMacros.CompareInt` (`.CurrentAmmo_28_752318D44ED93FAD5F9156BBE02568EF` (break `/Game/ShooterFighter/Blueprints/Structs/CharStruct` _structout))
    (:`==`
      (setmembers `/Game/ShooterFighter/Blueprints/Structs/CharStruct` :`StructRef` _char2info :`Reloading` true)
      (`KismetSystemLibrary.Delay` _reloadtime)
      (setmembers `/Game/ShooterFighter/Blueprints/Structs/CharStruct` :`StructRef` _char2info :`Reloading` false :`CurrentAmmo` (`.MaxAmmo_26_6C1A018E4C56911319A188845CCCC784` (break `/Game/ShooterFighter/Blueprints/Structs/CharStruct` (`self.Char2Info`)))))))

(event `Key|Up`
  (params (Key :type "Key Structure"))
  ;[1 1 1] P2 Input Chains
  (:`Pressed`
    (`self.SetInputChainP2` Key)))

(event `InputAction|Player2Jump`
  (params (Key :type "Key Structure"))
  (bind _char2 (`self.Char2`))
  (bind _inputenabled (`self.InputEnabled`))
  ;[1 1 1] Handle Jump 2P
  (:`Pressed`
    (if _inputenabled
      (bind _asbpcharacter_2 (cast `/Game/ShooterFighter/Blueprints/BPCharacter2` _char2))
      (`Character.Jump` _asbpcharacter_2)
      (bind _output_get (set `self.ActionState` "NewEnumerator2"))
      (`/Game/ShooterFighter/Blueprints/BPCharacter2.UpdateAnimation` _char2 _output_get)))
  (:`Released`
    (if _inputenabled
      (bind _asbpcharacter_2_2 (cast `/Game/ShooterFighter/Blueprints/BPCharacter2` _char2))
      (`Character.StopJumping` _asbpcharacter_2_2))))

(event `Key|Enter`
  (params (Key :type "Key Structure"))
  (bind _char2info (`self.Char2Info`))
  (bind (_movingr _shooting _reloading) (break `/Game/ShooterFighter/Blueprints/Structs/CharStruct` (`self.Char2Info`)))
  ;[1 1 1] Shooting 2P
  (:`Pressed`
    (`self.SetInputChainP2` Key)
    (if (and (`self.InputEnabled`) (not _shooting) (not _reloading))
      (`|ExecutionSequence`
        (:`then_0`
          (`GameplayStatics.PlaySoundAtLocation` "/Game/ShooterFighter/Sound/Effects/S_Gunshot.S_Gunshot" (0.0 0.0 0.0) (struct) 0.6))
        (:`then_1`
          (`|SpawnActorFromClass` "/Game/ShooterFighter/Blueprints/BP_Bullet_Player2.BP_Bullet_Player2_C" (`SceneComponent.K2_GetComponentToWorld` (`/Game/ShooterFighter/Blueprints/BPCharacter2.ArrowShot` (`self.Char2`))) "Undefined" "OverrideRootScale" null null))
        (:`then_2`
          (`self.UpdateAmmoP2`))
        (:`then_3`
          (setmembers `/Game/ShooterFighter/Blueprints/Structs/CharStruct` :`StructRef` _char2info :`Shooting` true)
          (`KismetSystemLibrary.Delay` (`.FireRate_8_44F8AAA74B17C0093544B193761FC9C2` (break `/Game/ShooterFighter/Blueprints/Structs/CharStruct` _char2info)))
          (setmembers `/Game/ShooterFighter/Blueprints/Structs/CharStruct` :`StructRef` _char2info :`Shooting` false))))))

(event `SpecialShotP2`
  (bind _char2info (`self.Char2Info`))
  (bind _returnvalue (`SceneComponent.K2_GetComponentToWorld` (`/Game/ShooterFighter/Blueprints/BPCharacter2.ArrowShot` (`self.Char2`))))
  ;[1 1 1] Special Shot P2
  (if (`self.InputEnabled`)
    (if (not (`.Reloading_5_2516DC3643F2DA088FF503800CA586F7` (break `/Game/ShooterFighter/Blueprints/Structs/CharStruct` (`self.Char2Info`))))
      (`|ExecutionSequence`
        (:`then_0`
          (`GameplayStatics.PlaySoundAtLocation` "/Game/ShooterFighter/Sound/Effects/S_Gunshot.S_Gunshot" (0.0 0.0 0.0) (struct) 0.6)
          (`|SpawnActorFromClass` "/Game/ShooterFighter/Blueprints/BP_Bullet_Player2.BP_Bullet_Player2_C" _returnvalue "Undefined" "OverrideRootScale" null null)
          (`self.UpdateAmmoP2`)
          (`KismetSystemLibrary.Delay` 0.15)
          (`GameplayStatics.PlaySoundAtLocation` "/Game/ShooterFighter/Sound/Effects/S_Gunshot.S_Gunshot" (0.0 0.0 0.0) (struct) 0.6)
          (`|SpawnActorFromClass` "/Game/ShooterFighter/Blueprints/BP_Bullet_Player2.BP_Bullet_Player2_C" _returnvalue "Undefined" "OverrideRootScale" null null))
        (:`then_1`
          (setmembers `/Game/ShooterFighter/Blueprints/Structs/CharStruct` :`StructRef` _char2info :`Shooting` true)
          (`KismetSystemLibrary.Delay` (+ (`.FireRate_8_44F8AAA74B17C0093544B193761FC9C2` (break `/Game/ShooterFighter/Blueprints/Structs/CharStruct` _char2info)) 0.15))
          (setmembers `/Game/ShooterFighter/Blueprints/Structs/CharStruct` :`StructRef` _char2info :`Shooting` false))))))

(event `InputAxis|Player2Right`
  (params (AxisValue :type "Float (single-precision)"))
  (bind _char2 (`self.Char2`))
  ;[1 1 1] Handle movement 2P
  (if (`self.InputEnabled`)
    (cast `/Game/ShooterFighter/Blueprints/BPCharacter2` _char2)
    (`Pawn.AddMovementInput` _char2 (1.0 0.0 0.0) AxisValue false)))

(event `Key|Down`
  (params (Key :type "Key Structure"))
  ;[1 1 1] P2 Input Chains
  (:`Pressed`
    (`self.SetInputChainP2` Key)))

(event `Key|Left`
  (params (Key :type "Key Structure"))
  ;[1 1 1] P2 Input Chains
  (:`Pressed`
    (`self.SetInputChainP2` Key)))

(event `OnLandedPlayer2`
  ;[1 1 1] Handle Jump 2P
  (bind _output_get (set `self.ActionState` "NewEnumerator0"))
  (`/Game/ShooterFighter/Blueprints/BPCharacter2.UpdateAnimation` (`self.Char2`) _output_get))

(event `Key|Right`
  (params (Key :type "Key Structure"))
  ;[1 1 1] P2 Input Chains
  (:`Pressed`
    (`self.SetInputChainP2` Key)))

(event `UpdateWinsP2`
  (bind _char2info (`self.Char2Info`))
  ;[1 1 1] Update Wins P2
  (setmembers `/Game/ShooterFighter/Blueprints/Structs/CharStruct` :`StructRef` _char2info :`CurrentWins` (+ (`.CurrentWins_30_FD63D54E4C90841E1CCF2E9FCAE436A6` (break `/Game/ShooterFighter/Blueprints/Structs/CharStruct` _char2info)) 1))
  (set `self.Round` (+ (`self.Round`) 1)))

(event `Respawn P2`
  (bind _char2info (`self.Char2Info`))
  (bind (_movingr _shooting _reloading _firerate _reloadtime _specialtimer _sm _inputchain _maxhealth _health _maxammo) (break `/Game/ShooterFighter/Blueprints/Structs/CharStruct` _char2info))
  ;[1 1 1] Respawn Player 2
  (setmembers `/Game/ShooterFighter/Blueprints/Structs/CharStruct` :`StructRef` _char2info :`Health` _maxhealth :`CurrentAmmo` _maxammo))

(event `DamageP2`
  (params (Damage :type "Float (double-precision)"))
  (bind _char2info (`self.Char2Info`))
  ;[1 1 1] Damage Player 2
  (setmembers `/Game/ShooterFighter/Blueprints/Structs/CharStruct` :`StructRef` _char2info :`Health` (- (`.Health_23_413A2251404E3EBFA307E59EFC07D439` (break `/Game/ShooterFighter/Blueprints/Structs/CharStruct` _char2info)) Damage)))

(fn `CheckIfSM_P1`
  (bind _char1info (`self.Char1Info`))
  (bind (_movingr _shooting _reloading _firerate _reloadtime _specialtimer _sm) (break `/Game/ShooterFighter/Blueprints/Structs/CharStruct` (`self.Char1Info`)))
  (bind (_movingr_2 _shooting_2 _reloading_2 _firerate_2 _reloadtime_2 _specialtimer_2 _sm_2 _inputchain) (break `/Game/ShooterFighter/Blueprints/Structs/CharStruct` (`self.Char1Info`)))
  (if _reloading
    _
    (elif (not _shooting)
      (for (_array_element _array_index) _sm
        (if (== (`|GetArrayItem` _inputchain) (break `/Game/ShooterFighter/Blueprints/SpecialMoves/SpecialMove` _array_element))
          (if (== (`|GetArrayItem` _inputchain 1) (`.Key2_4_977F2EFB4598B02B6BACCA8A38377FAC` (break `/Game/ShooterFighter/Blueprints/SpecialMoves/SpecialMove` _array_element)))
            (if (== (`|GetArrayItem` _inputchain 2) (`.Key3_6_7F0D8FC14FC8F51DFB10149B34CA9AFE` (break `/Game/ShooterFighter/Blueprints/SpecialMoves/SpecialMove` _array_element)))
              (`/Engine/EditorBlueprintResources/StandardMacros.CompareFloat` (- (.x (`self.K2_GetActorLocation` (`self.Char1`))) (.x (`self.K2_GetActorLocation` (`self.Char2`))))
                (:`>`
                  (if (== _array_index 1)
                    (setmembers `/Game/ShooterFighter/Blueprints/Structs/CharStruct` :`StructRef` _char1info :`Shooting` true)
                    (`self.SpecialMove1_P1`)
                    (setmembers `/Game/ShooterFighter/Blueprints/Structs/CharStruct` :`StructRef` (`self.Char1Info`) :`InputChain` (`|MakeArray` (`self.Nothing`) (`self.Nothing`) (`self.Nothing`)) :!label _label)))
                (:`<`
                  (if (== _array_index 0)
                    (setmembers `/Game/ShooterFighter/Blueprints/Structs/CharStruct` :`StructRef` _char1info :`Shooting` true)
                    (`self.SpecialMove1_P1`)
                    (goto _label)))))))))))

(fn `CheckIfSM_P2`
  (bind _char2info (`self.Char2Info`))
  (bind (_movingr _shooting _reloading _firerate _reloadtime _specialtimer _sm) (break `/Game/ShooterFighter/Blueprints/Structs/CharStruct` (`self.Char2Info`)))
  (bind (_movingr_2 _shooting_2 _reloading_2 _firerate_2 _reloadtime_2 _specialtimer_2 _sm_2 _inputchain) (break `/Game/ShooterFighter/Blueprints/Structs/CharStruct` (`self.Char2Info`)))
  (if (not (and _shooting _reloading))
    (for (_array_element _array_index) _sm
      (if (== (`|GetArrayItem` _inputchain) (break `/Game/ShooterFighter/Blueprints/SpecialMoves/SpecialMove` _array_element))
        (if (== (`|GetArrayItem` _inputchain 1) (`.Key2_4_977F2EFB4598B02B6BACCA8A38377FAC` (break `/Game/ShooterFighter/Blueprints/SpecialMoves/SpecialMove` _array_element)))
          (if (== (`|GetArrayItem` _inputchain 2) (`.Key3_6_7F0D8FC14FC8F51DFB10149B34CA9AFE` (break `/Game/ShooterFighter/Blueprints/SpecialMoves/SpecialMove` _array_element)))
            (`/Engine/EditorBlueprintResources/StandardMacros.CompareFloat` (- (.x (`self.K2_GetActorLocation` (`self.Char2`))) (.x (`self.K2_GetActorLocation` (`self.Char1`))))
              (:`>`
                (if (== _array_index 1)
                  (setmembers `/Game/ShooterFighter/Blueprints/Structs/CharStruct` :`StructRef` _char2info :`Shooting` true)
                  (`self.SpecialMove1_P2`)
                  (setmembers `/Game/ShooterFighter/Blueprints/Structs/CharStruct` :`StructRef` (`self.Char2Info`) :`InputChain` (`|MakeArray` (`self.Nothing`) (`self.Nothing`) (`self.Nothing`)) :!label _label)))
              (:`<`
                (if (== _array_index 0)
                  (setmembers `/Game/ShooterFighter/Blueprints/Structs/CharStruct` :`StructRef` _char2info :`Shooting` true)
                  (`self.SpecialMove1_P2`)
                  (goto _label))))))))))

(fn `SetInputChainP1`
  (params (keyPressed :type "Key Structure"))
  (bind _char1info (`self.Char1Info`))
  (bind _nothing (`self.Nothing`))
  (bind (_movingr _shooting _reloading _firerate _reloadtime _specialtimer _sm _inputchain) (break `/Game/ShooterFighter/Blueprints/Structs/CharStruct` (`self.Char1Info`)))
  (bind (_movingr_2 _shooting_2 _reloading_2 _firerate_2 _reloadtime_2 _specialtimer_2 _sm_2 _inputchain_2) (break `/Game/ShooterFighter/Blueprints/Structs/CharStruct` _char1info))
  (bind (_movingr_3 _shooting_3 _reloading_3 _firerate_3 _reloadtime_3 _specialtimer_3 _sm_3 _inputchain_3) (break `/Game/ShooterFighter/Blueprints/Structs/CharStruct` (`self.Char1Info`)))
  (if (> _specialtimer_3 0.0)
    (setmembers `/Game/ShooterFighter/Blueprints/Structs/CharStruct` :`StructRef` _char1info :`SpecialTimer` 0.5)
    (if (== (`|GetArrayItem` _inputchain_3) (`self.Nothing`))
      (`KismetArrayLibrary.Array_Set` _inputchain 0 keyPressed)
      (elif (== (`|GetArrayItem` _inputchain_2 1) (`self.Nothing`))
        (`KismetArrayLibrary.Array_Set` _inputchain 1 keyPressed)
        (elif (== (`|GetArrayItem` _inputchain_2 2) (`self.Nothing`))
          (`KismetArrayLibrary.Array_Set` _inputchain 2 keyPressed)
          (`self.CheckIfSM_P1`))))
    (else
      (setmembers `/Game/ShooterFighter/Blueprints/Structs/CharStruct` :`StructRef` (`self.Char1Info`) :`SpecialTimer` 0.5 :`InputChain` (`|MakeArray` keyPressed _nothing _nothing)))))

(fn `SetInputChainP2`
  (params (keyPressed :type "Key Structure"))
  (bind _char2info (`self.Char2Info`))
  (bind _nothing (`self.Nothing`))
  (bind (_movingr _shooting _reloading _firerate _reloadtime _specialtimer _sm _inputchain) (break `/Game/ShooterFighter/Blueprints/Structs/CharStruct` _char2info))
  (bind (_movingr_2 _shooting_2 _reloading_2 _firerate_2 _reloadtime_2 _specialtimer_2 _sm_2 _inputchain_2) (break `/Game/ShooterFighter/Blueprints/Structs/CharStruct` (`self.Char2Info`)))
  (if (> (`.SpecialTimer_12_4734324540203F26D7FC7C812F8E0032` (break `/Game/ShooterFighter/Blueprints/Structs/CharStruct` (`self.Char2Info`))) 0.0)
    (setmembers `/Game/ShooterFighter/Blueprints/Structs/CharStruct` :`StructRef` _char2info :`SpecialTimer` 0.5)
    (if (== (`|GetArrayItem` _inputchain) (`self.Nothing`))
      (`KismetArrayLibrary.Array_Set` _inputchain_2 0 keyPressed)
      (elif (== (`|GetArrayItem` _inputchain 1) (`self.Nothing`))
        (`KismetArrayLibrary.Array_Set` _inputchain_2 1 keyPressed)
        (elif (== (`|GetArrayItem` _inputchain 2) (`self.Nothing`))
          (`KismetArrayLibrary.Array_Set` _inputchain_2 2 keyPressed)
          (`self.CheckIfSM_P2`))))
    (else
      (setmembers `/Game/ShooterFighter/Blueprints/Structs/CharStruct` :`StructRef` _char2info :`SpecialTimer` 0.5 :`InputChain` (`|MakeArray` keyPressed _nothing _nothing)))))

(fn `UserConstructionScript`)