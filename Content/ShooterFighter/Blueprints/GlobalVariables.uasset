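; GlobalVariables is a Blueprint that manages a single 2D sound, stored as Music, through Play Sound and Stop Sound events.
; Play Sound stops any current Music, spawns the given sound with SpawnSound2D and stores the new component.
; Stop Sound stops the stored component if it is valid, so only one tracked sound plays at a time.
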(event `Stop Sound`
  (bind _music (`self.Music`))
  ;[1 1 1] Stop Sound
  (if (`KismetSystemLibrary.IsValid` _music)
    (`AudioComponent.Stop` _music)))

(event `Play Sound`
  (params (Sound :type "SoundBase Object Reference"))
  (bind _music (`self.Music`))
  ;[1 1 1] Play Sound
  (if (`KismetSystemLibrary.IsValid` _music)
    (`AudioComponent.Stop` _music))
  (bind _returnvalue (`GameplayStatics.SpawnSound2D` Sound 0.85))
  (set `self.Music` _returnvalue))