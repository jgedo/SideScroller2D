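; BPCharacter2 is the second player's sprite character in a shooter fighter, optionally moved by AI when the player controller flags it as AI-controlled with input enabled.
; Each tick it switches idle, walk and jump flipbooks by action state and turns to face the first BPCharacter found.
; The AI approaches beyond a horizontal distance threshold and backs away inside it.
; Landing notifies the controller, while AIShoot only makes a random comparison with nothing connected.
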(event `UpdateAnimation`
  (params (ActionState :type "/Game/ShooterFighter/Blueprints/Enums/Char_States Enum" :default "NewEnumerator0"))
  ;[1 1 1] Handle Animation
  (bind _output_get (set `self.ActionState` ActionState))
  (switch `/Game/ShooterFighter/Blueprints/Enums/Char_States` _output_get
    (:`NewEnumerator0`
      (`PaperFlipbookComponent.SetFlipbook` (`self.Sprite`) (select `bool` (> (`KismetMathLibrary.VSize` (`self.GetVelocity`)) 0.0) :`false` "/Game/ShooterFighter/Sprites/Flipbooks/Char2/FB_Idle-P2.FB_Idle-P2" :`true` "/Game/ShooterFighter/Sprites/Flipbooks/Char2/FB_Walking-P2.FB_Walking-P2" :!type "PaperFlipbook Object Reference")))
    (:`NewEnumerator1`
      (`PaperFlipbookComponent.SetFlipbook` (`self.Sprite`) "/Game/ShooterFighter/Sprites/Flipbooks/Char2/FB_Walking-P2.FB_Walking-P2"))
    (:`NewEnumerator2`
      (`PaperFlipbookComponent.SetFlipbook` (`self.Sprite`) "/Game/ShooterFighter/Sprites/Flipbooks/Char2/FB_Jump-P2.FB_Jump-P2"))))

(event `AIBehavior`
  (bind _pcontroller1 (`self.PController1`))
  (bind _returnvalue (- (.x (`self.K2_GetActorLocation` (`self.Char1`))) (.x (`self.K2_GetActorLocation`))))
  ;[1 1 1] AI Behavior
  (if (and (`/Game/ShooterFighter/Blueprints/MyPlayerController1.IsAIControlled` _pcontroller1) (`/Game/ShooterFighter/Blueprints/MyPlayerController1.InputEnabled` _pcontroller1))
    (`/Engine/EditorBlueprintResources/StandardMacros.CompareInt` (`KismetMathLibrary.Round` (`KismetMathLibrary.Abs` _returnvalue)) 100
      (:`>`
        (`self.AddMovementInput` (1.0 0.0 0.0) _returnvalue))
      (:`<`
        (`self.AddMovementInput` (-1.0 0.0 0.0) _returnvalue)))))

(event `AI Shoot`
  (`/Engine/EditorBlueprintResources/StandardMacros.CompareInt` (`KismetMathLibrary.RandomIntegerInRange` 0 100) 21))

(event `self.ReceiveBeginPlay`
  (`|ExecutionSequence`
    (:`then_0`
      (`ActorComponent.SetIsReplicated` (`self.Sprite`) true))
    (:`then_1`
      (bind _outactors (`GameplayStatics.GetAllActorsOfClass` "/Game/ShooterFighter/Blueprints/BPCharacter.BPCharacter_C"))
      (set `self.Char1` (`|GetArrayItem` _outactors)))
    (:`then_2`
      (bind _outactors_2 (`GameplayStatics.GetAllActorsOfClass` "/Game/ShooterFighter/Blueprints/MyPlayerController1.MyPlayerController1_C"))
      (set `self.PController1` (`|GetArrayItem` _outactors_2)))))

(event `self.ReceiveTick`
  (params (DeltaSeconds :type "Float (single-precision)"))
  ;[1 1 1] Tick - Updates animation
  (`self.AIBehavior`)
  (`self.UpdateAnimation` (`self.ActionState`))
  (`/Engine/EditorBlueprintResources/StandardMacros.CompareFloat` (- (.x (`self.K2_GetActorLocation`)) (.x (`self.K2_GetActorLocation` (`self.Char1`))))
    (:`>`
      (`self.K2_SetActorRotation` (`KismetMathLibrary.MakeRotator` 0.0 0.0 180.0)))
    (:`<`
      (`self.K2_SetActorRotation` (`KismetMathLibrary.MakeRotator` 0.0)))))

(event `self.OnLanded`
  (params (Hit :type "HitResult Structure (by ref)"))
  ;[1 1 1] Handle Jump
  (bind _asmy_player_controller_1 (cast `/Game/ShooterFighter/Blueprints/MyPlayerController1` (`self.PController1`)))
  (`/Game/ShooterFighter/Blueprints/MyPlayerController1.OnLandedPlayer2` _asmy_player_controller_1))

(fn `UserConstructionScript`)