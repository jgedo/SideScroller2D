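; Bullet actor for the shooter fighter game that reacts to overlaps on its Box component.
; The GameInstance's 1PCharacter value selects which character class it can hit and whether MyPlayerController1 applies a fixed damage amount to P1 or P2.
; It destroys itself on a character hit, or after a short delay on touching a BlockingVolume.
; Overlapping a BP_Bullet_Player2 destroys both bullets.
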(event `self.Box.OnComponentBeginOverlap`
  (params (OverlappedComponent :type "PrimitiveComponent Object Reference") (OtherActor :type "Actor Object Reference") (OtherComp :type "PrimitiveComponent Object Reference") (OtherBodyIndex :type Integer) (bFromSweep :type Boolean) (SweepResult :type "HitResult Structure (by ref)"))
  (bind _returnvalue (`GameplayStatics.GetPlayerController` 0))
  (`|ExecutionSequence`
    (:`then_0`
      (bind _asglobal_variables (cast `/Game/ShooterFighter/Blueprints/GlobalVariables` (`GameplayStatics.GetGameInstance`)))
      (switch `int` (`/Game/ShooterFighter/Blueprints/GlobalVariables.1P Character` _asglobal_variables)
        (:`1`
          (cast `/Game/ShooterFighter/Blueprints/BPCharacter2` OtherActor)
          (bind _asmy_player_controller_1 (cast `/Game/ShooterFighter/Blueprints/MyPlayerController1` _returnvalue))
          (`/Game/ShooterFighter/Blueprints/MyPlayerController1.DamageP2` _asmy_player_controller_1 0.08)
          (`self.K2_DestroyActor`))
        (:`2`
          (cast `/Game/ShooterFighter/Blueprints/BPCharacter` OtherActor)
          (bind _asmy_player_controller_1_2 (cast `/Game/ShooterFighter/Blueprints/MyPlayerController1` _returnvalue))
          (`/Game/ShooterFighter/Blueprints/MyPlayerController1.DamageP1` _asmy_player_controller_1_2 0.08)
          (`self.K2_DestroyActor`))))
    (:`then_1`
      (cast `BlockingVolume` OtherActor)
      (`KismetSystemLibrary.Delay` 0.5)
      (`self.K2_DestroyActor`))
    (:`then_2`
      (bind _asbp_bullet_player_2 (cast `/Game/ShooterFighter/Blueprints/BP_Bullet_Player2` OtherActor))
      (`self.K2_DestroyActor` _asbp_bullet_player_2)
      (`self.K2_DestroyActor`))))

(fn `UserConstructionScript`)