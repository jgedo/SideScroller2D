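; MyPlayerController1 is the first player's controller, which also sets up player two and handles horizontal movement.
; On BeginPlay it spawns a MyPlayerController2 and a BPCharacter2 at a hardcoded location, stores both, and has that controller possess the character.
; The MoveRight axis drives movement along world X when the controlled pawn is a BPCharacter, updating a MovingR facing flag from the input sign.
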(event `self.ReceiveBeginPlay`
  (bind _returnvalue (`KismetMathLibrary.MakeTransform` (250.0 495.0 152.0)))
  ;[1 1 1] Set Up Player 2
  (bind _returnvalue_2 (`|SpawnActorFromClass` "/Game/MyDemo/Blueprints/MyPlayerController2.MyPlayerController2_C" _returnvalue "Undefined" "OverrideRootScale" null null))
  (set `self.Char2Controller` _returnvalue_2)
  (bind _returnvalue_3 (`|SpawnActorFromClass` "/Game/MyDemo/Blueprints/BPCharacter2.BPCharacter2_C" _returnvalue "Undefined" "OverrideRootScale" null null))
  (set `self.Char2` _returnvalue_3)
  (`self.Possess` (`self.Char2Controller`) (`self.Char2`)))

(event `InputAxis|MoveRight`
  (params (AxisValue :type "Float (single-precision)"))
  (bind _returnvalue (`self.K2_GetPawn`))
  ;[1 1 1] Handle movement
  (cast `/Game/MyDemo/Blueprints/BPCharacter` _returnvalue)
  (if (> AxisValue 0.0)
    (set `self.MovingR` true)
    (elif (< AxisValue 0.0)
      (set `self.MovingR` false)))
  (`Pawn.AddMovementInput` _returnvalue (1.0 0.0 0.0) AxisValue false))

(fn `UserConstructionScript`)